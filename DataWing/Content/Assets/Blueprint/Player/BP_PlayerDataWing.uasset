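; Player actor that flies forward automatically in the Y-Z plane along Arrow1, steered by rolling with the MoveTurn axis.
; Each tick moves it with sweep, then line-traces behind it, setting a boosted speed when a static object is hit.
; Looping timers bleed speed while turning or braking, with holding both brakes adding a second reduction.
; Brake release or idle turn input can restore MaxSpeed unless the wall boost is active.
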(event `DetectWall`
  (bind _returnvalue (`self.K2_GetActorLocation`))
  ;[1 1 1] Touch Wall
  (bind (_outhit _returnvalue_2) (`KismetSystemLibrary.LineTraceSingleForObjects` :`Start` _returnvalue :`End` (+ _returnvalue (* (`SceneComponent.GetForwardVector` (`self.Arrow1`)) -350.0)) :`ObjectTypes` (`|MakeArray` "ObjectTypeQuery1" :!type "EObjectTypeQuery Enum") :`DrawDebugType` "ForOneFrame"))
  (if _returnvalue_2
    (set `self.Acceleration` true)
    (set `self.Speed` 20.0)
    (else
      (set `self.Acceleration` false))))

(event `InputAction|FreinL`
  (params (Key :type "Key Structure"))
  ;[1 1 1] Reduce on Turn
  (:`Pressed`
    (set `self.TimeEventRotate` 0.2 :!label _label)
    (set `self.PredictionTurnControllerReduce` true)
    (`KismetSystemLibrary.K2_SetTimerDelegate` (delegate `ReduceSpeedByRotate`) (`self.TimeEventRotate`) true))
  (:`Released`
    (set `self.TimeEventRotate` 0.0 :!label _label_2)
    (set `self.PredictionTurnControllerReduce` false)))

(event `InputAxis|MoveTurnReduce`
  (params (AxisValue :type "Float (single-precision)"))
  ;[1 1 1] Reduce on Turn
  (if (!= AxisValue 0.0)
    (`/Engine/EditorBlueprintResources/StandardMacros.DoOnce` false :!label _label_3
      (:`Completed`
        (goto _label)))
    (elif (== AxisValue 0.0)
      (if (not (`self.PredictionTurnControllerReduce`))
        (if (`KismetMathLibrary.BooleanNAND` (`self.FL`) (`self.RL`))
          (set `self.TimeEventRotate` 0.0)
          (if (not (`self.Acceleration`))
            (set `self.Speed` (`self.MaxSpeed`))
            (goto _label_3 :!via `Reset`)
            (else
              (goto _label_3 :!via `Reset`))))))))

(event `InputAction|FreinR`
  (params (Key :type "Key Structure"))
  ;[1 1 1] Reduce on Turn
  (:`Pressed`
    (goto _label))
  (:`Released`
    (goto _label_2)))

(event `self.ReceiveTick`
  (params (DeltaSeconds :type "Float (single-precision)"))
  (bind _speed (`self.Speed`))
  (bind (_returnvalue_x _returnvalue_y _returnvalue_z) (`KismetMathLibrary.BreakVector` (`SceneComponent.GetForwardVector` (`self.Arrow1`))))
  ;[1 1 1] Auto Walk
  (`self.K2_AddActorWorldOffset` (`KismetMathLibrary.MakeVector` 0.0 (* _returnvalue_y _speed) (* _returnvalue_z _speed)) true)
  (`self.DetectWall`))

(event `ReduceSpeedByRotate`
  ;[1 1 1] Reduce on Turn
  (if (!= (`self.TimeEventRotate`) 0.0)
    (if (>= (`self.Speed`) 0.1)
      (set `self.Speed` (- (`self.Speed`) 0.2)))))

(event `InputAction|FreinL`
  (params (Key :type "Key Structure"))
  ;[1 1 1] Frein Action
  (:`Pressed`
    (set `self.FL` true)
    (if (and (`self.FL`) (`self.RL`)) :!label _label_4
      (`self.LoopReduce` true)))
  (:`Released`
    (set `self.FL` false)
    (`self.LoopReduce` false)))

(event `InputAxis|MoveTurn`
  (params (AxisValue :type "Float (single-precision)"))
  (bind _returnvalue_roll (`KismetMathLibrary.BreakRotator` (`SceneComponent.K2_GetComponentRotation` (`self.Mesh`))))
  (bind _returnvalue_roll_2 (`KismetMathLibrary.BreakRotator` (`SceneComponent.K2_GetComponentRotation` (`self.Mesh`))))
  ;[1 1 1] Rotate Player
  (set `self.AxisRotate` AxisValue)
  (switch `int` (`KismetMathLibrary.FTrunc` (`self.AxisRotate`))
    (:`-1`
      (`KismetSystemLibrary.PrintString` "Gauche")
      (`self.K2_SetActorRotation` (`KismetMathLibrary.MakeRotator` (+ _returnvalue_roll_2 (`self.AxisRotate`)))))
    (:`0`
      (set `self.PredictionTurnControllerReduce` false))
    (:`1`
      (`KismetSystemLibrary.PrintString` "Droite")
      (`self.K2_SetActorRotation` (`KismetMathLibrary.MakeRotator` (+ _returnvalue_roll (`self.AxisRotate`)))))))

(event `LoopReduce`
  (params (`IsBreak?` :type Boolean))
  ;[1 1 1] Reduce speed by frein
  (if `IsBreak?`
    (set `self.TimeEventFrein` 0.2)
    (else
      (set `self.TimeEventFrein` 0.0)
      (if (not (`self.Acceleration`))
        (set `self.Speed` (`self.MaxSpeed`)))))
  (`KismetSystemLibrary.K2_SetTimerDelegate` (delegate `ReduceSpeedByFrein`) (`self.TimeEventFrein`) true))

(event `InputAction|FreinR`
  (params (Key :type "Key Structure"))
  ;[1 1 1] Frein Action
  (:`Pressed`
    (set `self.RL` true)
    (goto _label_4))
  (:`Released`
    (set `self.RL` false)
    (`self.LoopReduce` false)))

(event `ReduceSpeedByFrein`
  ;[1 1 1] Reduce speed by frein
  (if (>= (`self.Speed`) 0.1)
    (set `self.Speed` (- (`self.Speed`) 0.2))))

(fn `UserConstructionScript`)